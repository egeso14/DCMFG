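; AC_UIController is an actor component that drives combat UI for owners implementing BPI_UIController_Communicator.
; On BeginPlay it puts a screen-space direction indicator widget on the prototype character and forwards direction changes to it.
; A looping timer fills that widget's attack progress until the notify time, then drains it through the backswing.
; It also lazily creates and toggles a learned-moves combo menu, switching input mode and mouse cursor.
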(event `self.ReceiveBeginPlay`
  (if (`KismetSystemLibrary.DoesImplementInterface` (`self.GetOwner`) "/Game/Interfaces/BPI_UIController_Communicator.BPI_UIController_Communicator_C")
    (bind _returnvalue (`|CreateWidget` "/Game/UserInterface/WBP_DirectionIndicator.WBP_DirectionIndicator_C"))
    (set `self.DirectionalWidget` _returnvalue)
    (bind _asbp_prototype_character (cast `/Game/Custom_Characters/BP_PrototypeCharacter` (`self.GetOwner`)))
    (bind _returnvalue_2 (`|AddComponentByClass` _asbp_prototype_character "/Script/UMG.WidgetComponent" false (`KismetMathLibrary.MakeTransform` (0.0 0.0 0.0))))
    (`WidgetComponent.SetWidget` _returnvalue_2 (`self.DirectionalWidget`))
    (`WidgetComponent.SetWidgetSpace` _returnvalue_2 "Screen")
    (`/Game/UserInterface/WBP_DirectionIndicator.UpdateDirection` (`self.DirectionalWidget`) "NewEnumerator2")))

(event `/Game/Interfaces/BPI_UIController_Communicator.ReceiveDirectionUpdate`
  (params (newDirection :type "/Game/E_AttackDirections Enum" :default "NewEnumerator2"))
  (`/Game/UserInterface/WBP_DirectionIndicator.UpdateDirection` (`self.DirectionalWidget`) newDirection))

(event `/Game/Interfaces/BPI_UIController_Communicator.ReceiveAttackTimelineUpdate`
  (params (NotifyTime :type "Float (double-precision)") (AnimDuration :type "Float (double-precision)"))
  (set `self.AttackTimlineSwitch` NotifyTime)
  (set `self.AttackTimelineWindow` AnimDuration)
  (bind _returnvalue (`KismetSystemLibrary.K2_SetTimerDelegate` (delegate `TickAttackTImeline`) (`self.AttackTimelineUpdateRate`) true true))
  (set `self.AttackTimelineTimer` _returnvalue))

(event `TickAttackTImeline`
  (set `self.AttackTimelineRuntime` (+ (`self.AttackTimelineRuntime`) (`KismetSystemLibrary.K2_GetTimerElapsedTimeHandle` (`self.AttackTimelineTimer`))))
  (if (`self.Backswing`)
    (bind _output_get (set `self.AttackTimelineCurrentValue` (`KismetMathLibrary.Lerp` 1.0 0.0 (`KismetMathLibrary.FClamp` (/ (`self.AttackTimelineRuntime`) (- (`self.AttackTimelineWindow`) (`self.AttackTimlineSwitch`)))))))
    (`/Game/UserInterface/WBP_DirectionIndicator.UpdateAttackTimeline` (`self.DirectionalWidget`) _output_get)
    (if (== (`self.AttackTimelineCurrentValue`) 0.0)
      (`KismetSystemLibrary.K2_ClearAndInvalidateTimerHandle` (`self.AttackTimelineTimer`))
      (set `self.AttackTimelineRuntime` 0.0)
      (set `self.AttackTimelineCurrentValue` 0.0)
      (`/Game/UserInterface/WBP_DirectionIndicator.ClearProgress` (`self.DirectionalWidget`))
      (set `self.Backswing` false))
    (else
      (bind _output_get_2 (set `self.AttackTimelineCurrentValue` (`KismetMathLibrary.Lerp` 0.0 1.0 (`KismetMathLibrary.FClamp` (/ (`self.AttackTimelineRuntime`) (`self.AttackTimlineSwitch`))))))
      (`/Game/UserInterface/WBP_DirectionIndicator.UpdateAttackTimeline` (`self.DirectionalWidget`) _output_get_2)
      (if (== (`self.AttackTimelineCurrentValue`) 1.0)
        (set `self.Backswing` true)
        (set `self.AttackTimelineRuntime` 0.0)))))

(event `/Game/Interfaces/BPI_UIController_Communicator.ReceiveToggleComboMenu`
  (bind _returnvalue (`GameplayStatics.GetPlayerController` 0))
  (bind _returnvalue_2 (`GameplayStatics.GetPlayerController` 0))
  (bind (_returnvalue_x _returnvalue_y) (`KismetMathLibrary.BreakVector2D` (`WidgetLayoutLibrary.GetViewportSize`)))
  (bind _combomenuwidget (`self.ComboMenuWidget`))
  (if (`KismetSystemLibrary.DoesImplementInterface` (`self.GetOwner`) "/Game/Interfaces/BPI_UIController_Communicator.BPI_UIController_Communicator_C") :!label _label
    (`self.ComboMenuWidget`
      (:`then`
        (if (`Widget.IsInViewport` _combomenuwidget) :!label _label_2
          (`Widget.RemoveFromParent` _combomenuwidget)
          (`WidgetBlueprintLibrary.SetInputMode_GameOnly` _returnvalue)
          (set `PlayerController.bShowMouseCursor` false _returnvalue)
          (else
            (`UserWidget.AddToViewport` _combomenuwidget 0)
            (`WidgetBlueprintLibrary.SetInputMode_UIOnlyEx` _returnvalue_2 (`self.ComboMenuWidget`))
            (`PlayerController.SetMouseLocation` _returnvalue_2 (`KismetMathLibrary.FTrunc` (/ _returnvalue_x 2.0)) (`KismetMathLibrary.FTrunc` (/ _returnvalue_y 2.0)))
            (set `PlayerController.bShowMouseCursor` true _returnvalue_2))))
      (:`else`
        (`|ExecutionSequence`
          (:`then_0`
            (bind _returnvalue_3 (`|CreateWidget` "/Game/UserInterface/WBP_ComboMenu.WBP_ComboMenu_C"))
            (bind _output_get (set `self.ComboMenuWidget` _returnvalue_3))
            (`UserWidget.SetOwningPlayer` _output_get (`GameplayStatics.GetPlayerController` 0)))
          (:`then_1`
            (set `/Game/UserInterface/WBP_ComboMenu.LearnedMoves` (`self.Learned Moves`) (`self.ComboMenuWidget`)))
          (:`then_2`
            (goto _label_2)))))))

(event `/Game/Interfaces/BPI_UIController_Communicator.ReceiveComboMenuInfo`
  (params (LearnedMoves :type "/Game/Attacks/BPS_Movelist Structure"))
  (set `self.Learned Moves` LearnedMoves)
  (goto _label))