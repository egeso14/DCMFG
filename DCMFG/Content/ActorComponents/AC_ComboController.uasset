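; Actor component that manages eight-way attack direction and combo attack lookup for its owner.
; Left and right switch events cycle the direction with wraparound and notify the owner through BPI_DirectionListener.
; Attack triggers look up the current direction and combo number in nested moveset maps, sending attack data via BPI_AttackDataListener; nothing here increments the combo.
; BeginPlay fills every direction with copies of a placeholder debug moveset through macros.
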(event `self.ReceiveBeginPlay`
  (`self.InitializeDirectionAttacksMap`))

(event `/Game/Interfaces/BPI_InputListener.OnRightSwitchTriggered`
  (bind _returnvalue (`self.GetOwner`))
  (if (> (`self.currentDirection`) 6)
    (set `self.currentDirection` "NewEnumerator2")
    (else
      (set `self.currentDirection` (cast `/Game/E_AttackDirections` (+ (`self.currentDirection`) 1)))))
  (`KismetSystemLibrary.PrintString` (`|GetEnumeratorNameAsString` (`self.currentDirection`)) :!label _label)
  (if (`KismetSystemLibrary.DoesImplementInterface` _returnvalue "/Game/Interfaces/BPI_DirectionListener.BPI_DirectionListener_C")
    (message `/Game/Interfaces/BPI_DirectionListener.OnDirectionChanged` _returnvalue (`self.currentDirection`))))

(event `/Game/Interfaces/BPI_InputListener.OnLeftSwitchTriggered`
  (if (< (`self.currentDirection`) 1)
    (set `self.currentDirection` "NewEnumerator1")
    (goto _label)
    (else
      (set `self.currentDirection` (cast `/Game/E_AttackDirections` (- (`self.currentDirection`) 1)))
      (goto _label))))

(event `/Game/Interfaces/BPI_InputListener.OnAttackTriggered`
  (bind _returnvalue (`self.GetOwner`))
  (bind _exists (`self.ComboSequenceNumberExistsInDirection` (`self.comboNumber`) (`self.currentDirection`)))
  (if _exists
    (bind _attack (`self.GetNextAttackInfo`))
    (if (`KismetSystemLibrary.DoesImplementInterface` _returnvalue "/Game/Interfaces/BPI_AttackDataListener.BPI_AttackDataListener_C")
      (message `/Game/Interfaces/BPI_AttackDataListener.OnAttackDataSent` _returnvalue _attack)
      (`KismetSystemLibrary.PrintString` (`KismetStringLibrary.Concat_StrStr` "Sent attack data is this: " (`/Game/Attacks/DA_Attack.Name` _attack)))
      (else
        (`KismetSystemLibrary.PrintString` "Owner does not implement correct interface")))))

(fn `ComboSequenceNumberExistsInDirection`
  (params (ComboNumber :type Integer) (Direction :type "/Game/E_AttackDirections Enum" :default "NewEnumerator2"))
  (returns (Exists :type Boolean))
  (bind (_value _returnvalue) (`BlueprintMapLibrary.Map_Find` (`.DirectionMovesets_4_49FF136C44257DF9DFAF6284629AB469` (break `/Game/Attacks/BPS_MasterMoveset` (`self.MasterMoveset`))) Direction))
  (if _returnvalue
    (return (`.ReturnValue` (`BlueprintMapLibrary.Map_Find` (`.AttackEntries_6_1C1EC3C14DDB661A9956E89A3B400320` (break `/Game/Attacks/BPS_DirectionMoveset` _value)) ComboNumber)))
    (else
      (`KismetSystemLibrary.PrintText` "Direction not in MasterMoveset"))))

(fn `GetNextAttackInfo`
  (returns (Attack :type "/Game/Attacks/DA_Attack Object Reference"))
  (return (`BlueprintMapLibrary.Map_Find` (`.AttackEntries_6_1C1EC3C14DDB661A9956E89A3B400320` (break `/Game/Attacks/BPS_DirectionMoveset` (`BlueprintMapLibrary.Map_Find` (`.DirectionMovesets_4_49FF136C44257DF9DFAF6284629AB469` (break `/Game/Attacks/BPS_MasterMoveset` (`self.MasterMoveset`))) (`self.currentDirection`)))) (`self.comboNumber`))))

(fn `InitializeDirectionAttacksMap`
  (bind _directionmovesets (break `/Game/Attacks/BPS_MasterMoveset` (`self.MasterMoveset`)))
  ; Puts debug moves into the debug moveset that is used for testing until real attack assets and moveset building systems are made
  (for _index (range 4)
    (`BlueprintMapLibrary.Map_Add` (`.AttackEntries_6_1C1EC3C14DDB661A9956E89A3B400320` (break `/Game/Attacks/BPS_DirectionMoveset` (`self.DebugMoveset`))) _index "/Game/Attacks/DA_DebugAttack.DA_DebugAttack"))
  (bind _enumvalue (foreach `/Game/E_AttackDirections` false)
    (:`LoopBody`
      (switch `/Game/E_AttackDirections` _enumvalue
        (:`NewEnumerator2`
          ; Fills each direction moveset with a copy of the moves contained within the debug moveset
          (bind (_keypin _valuepin) (`|MapForEach` (`.AttackEntries_6_1C1EC3C14DDB661A9956E89A3B400320` (break `/Game/Attacks/BPS_DirectionMoveset` (`self.DebugMoveset`))))
            (:`then`
              (`BlueprintMapLibrary.Map_Add` (`.AttackEntries_6_1C1EC3C14DDB661A9956E89A3B400320` (break `/Game/Attacks/BPS_DirectionMoveset` (`self.TopMoveset`))) _keypin _valuepin))
            (:`CompletedPin`
              ; Fills the directional values of the master moveset with each directional movset
              (`BlueprintMapLibrary.Map_Add` _directionmovesets _enumvalue (`self.TopMoveset`)))))
        (:`NewEnumerator3`
          (bind (_keypin_2 _valuepin_2) (`|MapForEach` (`.AttackEntries_6_1C1EC3C14DDB661A9956E89A3B400320` (break `/Game/Attacks/BPS_DirectionMoveset` (`self.DebugMoveset`))))
            (:`then`
              (`BlueprintMapLibrary.Map_Add` (`.AttackEntries_6_1C1EC3C14DDB661A9956E89A3B400320` (break `/Game/Attacks/BPS_DirectionMoveset` (`self.TopRightMoveset`))) _keypin_2 _valuepin_2))
            (:`CompletedPin`
              (`BlueprintMapLibrary.Map_Add` _directionmovesets _enumvalue (`self.TopRightMoveset`)))))
        (:`NewEnumerator4`
          (bind (_keypin_3 _valuepin_3) (`|MapForEach` (`.AttackEntries_6_1C1EC3C14DDB661A9956E89A3B400320` (break `/Game/Attacks/BPS_DirectionMoveset` (`self.DebugMoveset`))))
            (:`then`
              (`BlueprintMapLibrary.Map_Add` (`.AttackEntries_6_1C1EC3C14DDB661A9956E89A3B400320` (break `/Game/Attacks/BPS_DirectionMoveset` (`self.RightMoveset`))) _keypin_3 _valuepin_3))
            (:`CompletedPin`
              (`BlueprintMapLibrary.Map_Add` _directionmovesets _enumvalue (`self.RightMoveset`)))))
        (:`NewEnumerator5`
          (bind (_keypin_4 _valuepin_4) (`|MapForEach` (`.AttackEntries_6_1C1EC3C14DDB661A9956E89A3B400320` (break `/Game/Attacks/BPS_DirectionMoveset` (`self.DebugMoveset`))))
            (:`then`
              (`BlueprintMapLibrary.Map_Add` (`.AttackEntries_6_1C1EC3C14DDB661A9956E89A3B400320` (break `/Game/Attacks/BPS_DirectionMoveset` (`self.BottomRightMoveset`))) _keypin_4 _valuepin_4))
            (:`CompletedPin`
              (`BlueprintMapLibrary.Map_Add` _directionmovesets _enumvalue (`self.BottomRightMoveset`)))))
        (:`NewEnumerator6`
          (bind (_keypin_5 _valuepin_5) (`|MapForEach` (`.AttackEntries_6_1C1EC3C14DDB661A9956E89A3B400320` (break `/Game/Attacks/BPS_DirectionMoveset` (`self.DebugMoveset`))))
            (:`then`
              (`BlueprintMapLibrary.Map_Add` (`.AttackEntries_6_1C1EC3C14DDB661A9956E89A3B400320` (break `/Game/Attacks/BPS_DirectionMoveset` (`self.BottomMoveset`))) _keypin_5 _valuepin_5))
            (:`CompletedPin`
              (`BlueprintMapLibrary.Map_Add` _directionmovesets _enumvalue (`self.BottomMoveset`)))))
        (:`NewEnumerator7`
          (bind (_keypin_6 _valuepin_6) (`|MapForEach` (`.AttackEntries_6_1C1EC3C14DDB661A9956E89A3B400320` (break `/Game/Attacks/BPS_DirectionMoveset` (`self.DebugMoveset`))))
            (:`then`
              (`BlueprintMapLibrary.Map_Add` (`.AttackEntries_6_1C1EC3C14DDB661A9956E89A3B400320` (break `/Game/Attacks/BPS_DirectionMoveset` (`self.BottomLeftMoveset`))) _keypin_6 _valuepin_6))
            (:`CompletedPin`
              (`BlueprintMapLibrary.Map_Add` _directionmovesets _enumvalue (`self.BottomLeftMoveset`)))))
        (:`NewEnumerator0`
          (bind (_keypin_7 _valuepin_7) (`|MapForEach` (`.AttackEntries_6_1C1EC3C14DDB661A9956E89A3B400320` (break `/Game/Attacks/BPS_DirectionMoveset` (`self.DebugMoveset`))))
            (:`then`
              (`BlueprintMapLibrary.Map_Add` (`.AttackEntries_6_1C1EC3C14DDB661A9956E89A3B400320` (break `/Game/Attacks/BPS_DirectionMoveset` (`self.LeftMoveset`))) _keypin_7 _valuepin_7))
            (:`CompletedPin`
              (`BlueprintMapLibrary.Map_Add` _directionmovesets _enumvalue (`self.LeftMoveset`)))))
        (:`NewEnumerator1`
          (bind (_keypin_8 _valuepin_8) (`|MapForEach` (`.AttackEntries_6_1C1EC3C14DDB661A9956E89A3B400320` (break `/Game/Attacks/BPS_DirectionMoveset` (`self.DebugMoveset`))))
            (:`then`
              (`BlueprintMapLibrary.Map_Add` (`.AttackEntries_6_1C1EC3C14DDB661A9956E89A3B400320` (break `/Game/Attacks/BPS_DirectionMoveset` (`self.TopLeftMoveset`))) _keypin_8 _valuepin_8))
            (:`CompletedPin`
              (`BlueprintMapLibrary.Map_Add` _directionmovesets _enumvalue (`self.TopLeftMoveset`)))))))))

(fn `ResetCombo`
  (set `self.comboNumber` 1))