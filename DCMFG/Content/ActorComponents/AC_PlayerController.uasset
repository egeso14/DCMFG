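; AC_PlayerController is an actor component that routes player input to its owning BP_PrototypeCharacter.
; On BeginPlay it casts the owner, gets its PlayerController and adds IMC_Default to the Enhanced Input subsystem.
; Attack, switch-left and switch-right actions are forwarded to the owner as BPI_InputListener interface messages, with debug prints along the way.
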(event `self.ReceiveBeginPlay`
  (bind _asbp_prototype_character (cast `/Game/Custom_Characters/BP_PrototypeCharacter` (`self.GetOwner`)))
  (bind _asplayer_controller (cast `PlayerController` (`Pawn.GetController` _asbp_prototype_character))
    (:`then`
      (`EnhancedInputSubsystemInterface.AddMappingContext` (pcsubsystem `EnhancedInputLocalPlayerSubsystem` _asplayer_controller) "/Game/Input/IMC_Default.IMC_Default" 0 (struct)))
    (:`CastFailed`
      (`KismetSystemLibrary.PrintText` "Cast to player controller failed"))))

(event `EnhancedInput|/Game/Input/Actions/IA_Attack`
  (params (ActionValue :type Boolean) (ElapsedSeconds :type "Float (double-precision)") (TriggeredSeconds :type "Float (double-precision)") (InputAction :type "InputAction Object Reference" :default "/Game/Input/Actions/IA_Attack.IA_Attack"))
  (bind _returnvalue (`self.GetOwner`))
  (:`Triggered`
    (if (`KismetSystemLibrary.DoesImplementInterface` _returnvalue "/Game/Interfaces/BPI_InputListener.BPI_InputListener_C")
      (message `/Game/Interfaces/BPI_InputListener.OnAttackTriggered` _returnvalue)
      (`KismetSystemLibrary.PrintString` "Attack input registered by controller")
      (else
        (`KismetSystemLibrary.PrintString` "Object doesn't implement required interface")))))

(event `EnhancedInput|/Game/Input/Actions/IA_SwitchLeft`
  (params (ActionValue :type Boolean) (ElapsedSeconds :type "Float (double-precision)") (TriggeredSeconds :type "Float (double-precision)") (InputAction :type "InputAction Object Reference" :default "/Game/Input/Actions/IA_SwitchLeft.IA_SwitchLeft"))
  (bind _returnvalue (`self.GetOwner`))
  (:`Triggered`
    (if (`KismetSystemLibrary.DoesImplementInterface` _returnvalue "/Game/Interfaces/BPI_InputListener.BPI_InputListener_C")
      (message `/Game/Interfaces/BPI_InputListener.OnLeftSwitchTriggered` _returnvalue))))

(event `EnhancedInput|/Game/Input/Actions/IA_SwitchRight`
  (params (ActionValue :type Boolean) (ElapsedSeconds :type "Float (double-precision)") (TriggeredSeconds :type "Float (double-precision)") (InputAction :type "InputAction Object Reference" :default "/Game/Input/Actions/IA_SwitchRight.IA_SwitchRight"))
  (bind _returnvalue (`self.GetOwner`))
  (:`Triggered`
    (if (`KismetSystemLibrary.DoesImplementInterface` _returnvalue "/Game/Interfaces/BPI_InputListener.BPI_InputListener_C")
      (message `/Game/Interfaces/BPI_InputListener.OnRightSwitchTriggered` _returnvalue)
      (`KismetSystemLibrary.PrintString` "Controller component sent attack trigger to characrter"))))