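; BP_PrototypeCharacter is a combat character that acts as a message hub between its controller components and its animation Blueprint.
; It forwards switch and attack input to the combo and stance controllers, and attack data to the attack controller.
; Animation notifies feed back to the combo controller, timeline and direction updates reach the UI controller, and stance changes reach the anim instance cached on BeginPlay.
; All relays are interface-checked, some with optional debug printing.
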(event `self.ReceiveBeginPlay`
  (bind _returnvalue (`SkeletalMeshComponent.GetAnimInstance` (`self.Mesh`)))
  (if (`KismetSystemLibrary.IsValid` _returnvalue)
    (bind _asabp_prototype_complete (cast `/Game/AnimationControllers/ABP_PrototypeComplete` _returnvalue))
    (set `self.AnimationBP` _asabp_prototype_complete)
    (else
      (`KismetSystemLibrary.PrintString` "Animation instance was invalid"))))

(event `/Game/Interfaces/BPI_UIController_Communicator.AttackTimelineUpdate`
  (params (NotifyTime :type "Float (double-precision)") (AnimDuration :type "Float (double-precision)"))
  (bind _ac_uicontroller (`self.AC_UIController`))
  (if (`KismetSystemLibrary.DoesImplementInterface` _ac_uicontroller "/Game/Interfaces/BPI_UIController_Communicator.BPI_UIController_Communicator_C")
    (`/Game/Interfaces/BPI_UIController_Communicator.AttackTimelineUpdate` _ac_uicontroller NotifyTime AnimDuration)))

(event `/Game/Interfaces/BPI_InputListener.OnLeftSwitchTriggered`
  (bind _ac_combocontroller (`self.AC_ComboController`))
  (if (`KismetSystemLibrary.DoesImplementInterface` _ac_combocontroller "/Game/Interfaces/BPI_InputListener.BPI_InputListener_C")
    (`/Game/ActorComponents/AC_ComboController.OnLeftSwitchTriggered` _ac_combocontroller)
    (if (`self.DebugTextOutputs`)
      (`KismetSystemLibrary.PrintString` (`KismetStringLibrary.Concat_StrStr` (`KismetSystemLibrary.GetDisplayName` self) " sent Left Switch Input to " (`KismetSystemLibrary.GetDisplayName` (`self.AC_ComboController`)))))
    (elif (`self.DebugTextOutputs`)
      (`KismetSystemLibrary.PrintString` (`KismetStringLibrary.Concat_StrStr` (`KismetSystemLibrary.GetDisplayName` self) "'s " (`KismetSystemLibrary.GetDisplayName` (`self.AC_ComboController`)) " does not implement the BPI Attack Data interface")))))

(event `/Game/Interfaces/BPI_InputListener.OnRightSwitchTriggered`
  (bind _ac_combocontroller (`self.AC_ComboController`))
  (if (`KismetSystemLibrary.DoesImplementInterface` _ac_combocontroller "/Game/Interfaces/BPI_InputListener.BPI_InputListener_C")
    (`/Game/ActorComponents/AC_ComboController.OnRightSwitchTriggered` _ac_combocontroller)
    (if (`self.DebugTextOutputs`)
      (`KismetSystemLibrary.PrintString` (`KismetStringLibrary.Concat_StrStr` (`KismetSystemLibrary.GetDisplayName` self) " sent Right Switch Input to " (`KismetSystemLibrary.GetDisplayName` (`self.AC_ComboController`)))))
    (elif (`self.DebugTextOutputs`)
      (`KismetSystemLibrary.PrintString` (`KismetStringLibrary.Concat_StrStr` (`KismetSystemLibrary.GetDisplayName` self) "'s " (`KismetSystemLibrary.GetDisplayName` (`self.AC_ComboController`)) " does not implement the BPI Attack Data interface")))))

(event `/Game/Interfaces/BPI_InputListener.OnAttackTriggered`
  (bind _ac_combocontroller (`self.AC_ComboController`))
  (if (`KismetSystemLibrary.DoesImplementInterface` _ac_combocontroller "/Game/Interfaces/BPI_InputListener.BPI_InputListener_C")
    (`/Game/Interfaces/BPI_InputListener.OnAttackTriggered` _ac_combocontroller)
    (if (`self.DebugTextOutputs`)
      (`KismetSystemLibrary.PrintString` (`KismetStringLibrary.Concat_StrStr` (`KismetSystemLibrary.GetDisplayName` self) " sent Attack Input to " (`KismetSystemLibrary.GetDisplayName` (`self.AC_ComboController`)))))
    (elif (`self.DebugTextOutputs`)
      (`KismetSystemLibrary.PrintString` (`KismetStringLibrary.Concat_StrStr` (`KismetSystemLibrary.GetDisplayName` self) "'s " (`KismetSystemLibrary.GetDisplayName` (`self.AC_ComboController`)) " does not implement the BPI Attack Data interface")))))

(event `/Game/Interfaces/BPI_AttackDataListener.OnAttackDataSent`
  (params (Attack :type "/Game/Attacks/DA_Attack Object Reference"))
  (bind _ac_attackcontroller (`self.AC_AttackController`))
  (if (`KismetSystemLibrary.DoesImplementInterface` _ac_attackcontroller "/Game/Interfaces/BPI_AttackDataListener.BPI_AttackDataListener_C")
    (`/Game/Interfaces/BPI_AttackDataListener.OnAttackDataSent` _ac_attackcontroller Attack)
    (if (`self.DebugTextOutputs`)
      (`KismetSystemLibrary.PrintString` (`KismetStringLibrary.Concat_StrStr` (`KismetSystemLibrary.GetDisplayName` self) " sent Attack data for " (`/Game/Attacks/DA_Attack.Name` Attack) " to " (`KismetSystemLibrary.GetDisplayName` (`self.AC_AttackController`)))))
    (elif (`self.DebugTextOutputs`)
      (`KismetSystemLibrary.PrintString` (`KismetStringLibrary.Concat_StrStr` (`KismetSystemLibrary.GetDisplayName` self) "'s " (`KismetSystemLibrary.GetDisplayName` (`self.AC_AttackController`)) " does not implement the BPI Attack Data interface")))))

(event `/Game/Interfaces/BPI_UIController_Communicator.OnDirectionChanged`
  (params (newDirection :type "/Game/E_AttackDirections Enum" :default "NewEnumerator2"))
  (bind _ac_uicontroller (`self.AC_UIController`))
  (if (`KismetSystemLibrary.DoesImplementInterface` _ac_uicontroller "/Game/Interfaces/BPI_UIController_Communicator.BPI_UIController_Communicator_C")
    (`/Game/Interfaces/BPI_UIController_Communicator.OnDirectionChanged` _ac_uicontroller newDirection)))

(event `/Game/Interfaces/BPI_AttackDataListener.UpdateFromAttackAnim`
  (params (Attack :type "/Game/Attacks/DA_Attack Object Reference") (TriggeredNotify :type Name))
  (bind _ac_combocontroller (`self.AC_ComboController`))
  (if (`KismetSystemLibrary.DoesImplementInterface` _ac_combocontroller "/Game/Interfaces/BPI_AttackDataListener.BPI_AttackDataListener_C")
    (`/Game/Interfaces/BPI_AttackDataListener.UpdateFromAttackAnim` _ac_combocontroller Attack TriggeredNotify)))

(event `/Game/Interfaces/BPI_InputListener.OnStanceSwitchTriggered`
  (if (`KismetSystemLibrary.DoesImplementInterface` (`self.AC_StanceController`) "/Game/Interfaces/BPI_InputListener.BPI_InputListener_C")
    (`/Game/Interfaces/BPI_InputListener.OnStanceSwitchTriggered` (`self.AC_StanceController`))))

(event `/Game/Interfaces/BPI_StanceListener.OnStanceChange`
  (params (NewStance :type "/Game/E_Stances Enum" :default "NewEnumerator0"))
  (bind _animationbp (`self.AnimationBP`))
  (if (`KismetSystemLibrary.DoesImplementInterface` _animationbp "/Game/Interfaces/BPI_StanceListener.BPI_StanceListener_C")
    (`/Game/AnimationControllers/ABP_PrototypeComplete.OnStanceChange` _animationbp NewStance)))

(fn `UserConstructionScript`
  (`parent.UserConstructionScript`))